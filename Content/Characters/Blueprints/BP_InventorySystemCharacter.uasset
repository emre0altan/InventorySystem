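; Player character Blueprint that creates the game HUD and inventory panel and toggles between them with Tab, locking move and look input while the inventory is open.
; Opening fills weapon, head, torso and pants tiles from Inventory's owned items and sets the SceneCapture show-only list for the character preview.
; Tick recaptures that preview while the panel is open.
; OnOwnedItemsUpdate re-enters the tile refresh path, which also sets the open flag.
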(event `self.ReceiveBeginPlay`
  ;[1 1 1] Initialization
  (bind _returnvalue (`|CreateWidget` "/Game/UI/Widget_GamePanel.Widget_GamePanel_C"))
  (bind _output_get (set `self.GamePanel` _returnvalue))
  (`UserWidget.AddToViewport` _output_get 0)
  (bind _returnvalue_2 (`|CreateWidget` "/Game/UI/Widget_InventoryPanel.Widget_InventoryPanel_C"))
  (set `self.InventoryPanel` _returnvalue_2)
  (set `self.PlayerController` (`GameplayStatics.GetPlayerController` 0))
  (bind _asbp_inventory_system_character (cast `/Game/Characters/Blueprints/BP_InventorySystemCharacter` (`GameplayStatics.GetPlayerCharacter` 0)))
  (set `self.PlayerCharacter` _asbp_inventory_system_character))

(event `Key|Tab`
  (params (Key :type "Key Structure"))
  (bind _inventorypanel (`self.InventoryPanel`))
  (bind _playercontroller (`self.PlayerController`))
  (bind _inventorypanel_2 (`self.InventoryPanel`))
  (bind _inventory (`self.Inventory`))
  (bind _gamepanel (`self.GamePanel`))
  (bind _array (`|MakeArray` (`self.PlayerCharacter`) (`CharacterInventory.CurrentWeaponItem` (`self.Inventory`)) :!type "Actor Object Reference"))
  ;[1 1 1] Inventory Panel
  (:`Pressed`
    (`/Engine/EditorBlueprintResources/StandardMacros.FlipFlop`
      (:`A`
        (`Widget.RemoveFromParent` _gamepanel)
        (`UserWidget.AddToViewport` _inventorypanel 0)
        (`Controller.SetIgnoreMoveInput` _playercontroller true)
        (`Controller.SetIgnoreLookInput` _playercontroller true)
        (set `PlayerController.bShowMouseCursor` true _playercontroller)
        (`ListView.BP_SetListItems` (`/Game/UI/Widget_InventoryPanel.WeaponsTile` _inventorypanel_2) (`CharacterInventory.OwnedWeaponItemDatas` _inventory) :!label _label)
        (`ListView.BP_SetListItems` (`/Game/UI/Widget_InventoryPanel.HeadsTile` _inventorypanel_2) (`CharacterInventory.OwnedHeadItemDatas` _inventory))
        (`ListView.BP_SetListItems` (`/Game/UI/Widget_InventoryPanel.TorsoTile` _inventorypanel_2) (`CharacterInventory.OwnedTorsoItemDatas` _inventory))
        (`ListView.BP_SetListItems` (`/Game/UI/Widget_InventoryPanel.PantsTile` _inventorypanel_2) (`CharacterInventory.OwnedPantsItemDatas` _inventory))
        (set `self.IsInventoryPanelOpen` true)
        (for _array_element (`InventorySystemCharacter.SidePlanesForPreview` (`self.PlayerCharacter`))
          (`KismetArrayLibrary.Array_Append` _array (`|MakeArray` _array_element)))
        (set `SceneCaptureComponent.ShowOnlyActors` _array (`self.SceneCaptureComponent`)))
      (:`B`
        (`UserWidget.AddToViewport` _gamepanel 0)
        (`Widget.RemoveFromParent` _inventorypanel)
        (`Controller.ResetIgnoreMoveInput` _playercontroller)
        (`Controller.ResetIgnoreLookInput` _playercontroller)
        (set `PlayerController.bShowMouseCursor` false _playercontroller)
        (set `self.IsInventoryPanelOpen` false)))))

(event `self.OnOwnedItemsUpdate`
  ;[1 1 1] Inventory Panel
  (goto _label))

(event `self.ReceiveTick`
  (params (DeltaSeconds :type "Float (single-precision)"))
  (if (`self.IsInventoryPanelOpen`)
    (`SceneCaptureComponent2D.CaptureScene` (`InventorySystemCharacter.SceneCaptureComponent` (`self.PlayerCharacter`)))))

(fn `UserConstructionScript`)